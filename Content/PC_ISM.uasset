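; PC_ISM procedurally builds a 200×200×200 grid of instanced static mesh instances, eight million in total.
; Each Tick spawns a new A_ISM actor for one Z layer until all layers exist, spreading the work across frames.
; Nested loops fill a transform array on 256-unit spacing, which goes to that actor's ISMC in one batched local-space AddInstances call before being cleared.
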(event `self.ReceiveBeginPlay`)

(event `self.ReceiveTick`
  (params (DeltaSeconds :type "Float (single-precision)"))
  (if (< (`self.Z`) 200)
    (bind _returnvalue (`|SpawnActorFromClass` "/Game/A_ISM.A_ISM_C" (`KismetMathLibrary.MakeTransform` (0.0 0.0 0.0)) "AlwaysSpawn" "MultiplyWithRoot" self null))
    (set `self.AISM` _returnvalue)
    (for _index (range 200)
      (for _index_2 (range 200)
        (`KismetArrayLibrary.Array_Add` (`self.InstancesTransforms`) (`KismetMathLibrary.MakeTransform` (* (`KismetMathLibrary.MakeVector` (`KismetMathLibrary.Conv_IntToDouble` _index_2) (`KismetMathLibrary.Conv_IntToDouble` _index) (+ (`KismetMathLibrary.Conv_IntToDouble` (`self.Z`)) 0.5)) (256.0 256.0 256.0))))))
    (`InstancedStaticMeshComponent.AddInstances` (`/Game/A_ISM.ISMC` (`self.AISM`)) (`self.InstancesTransforms`) false false)
    (`KismetArrayLibrary.Array_Clear` (`self.InstancesTransforms`))
    (`/Engine/EditorBlueprintResources/StandardMacros.IncrementInt` (`self.Z`))))

(fn `UserConstructionScript`)